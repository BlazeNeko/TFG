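; AI controller for a plane that drives its obstacle avoidance through a Behavior Tree.
; On BeginPlay it sets up Plane_Blackboard and runs PlaneBT.
; Every Tick it calls UseBlackboard again and copies the Avoid flag from the controlled pawn's SensorComponent into the blackboard's Avoid key.
; An unconnected test chain with delays, StopMovement and Avoid resets never runs.
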(event EventBeginPlay
  ;[0.231 1 0.6818] Inicializar Behaviour Tree
  (Class|AIController|UseBlackboard "/Game/Blueprints/BT/Plane_Blackboard.Plane_Blackboard")
  (AI|RunBehaviorTree "/Game/Blueprints/BT/PlaneBT.PlaneBT"))

(event EventTick
  (params (DeltaSeconds :type Float%20%28single-precision%29))
  ;[1 1 1] Actualiza los valores de la pizarra relacionados con evitar obstáculos en cada tick.
  (bind _blackboardcomponent (Class|AIController|UseBlackboard "/Game/Blueprints/BT/Plane_Blackboard.Plane_Blackboard"))
  (AI|Components|Blackboard|SetValueasBool _blackboardcomponent (Utilities|Name|MakeLiteralName "Avoid") (Variables|/Script/TFG.SensorComponent|Getavoid (Actor|GetComponentbyClass (Pawn|GetControlledPawn) "/Script/TFG.SensorComponent"))))

(fn ConstructionScript)